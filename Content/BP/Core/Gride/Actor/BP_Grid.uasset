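; Tile grid actor that builds a ground-conforming grid in its construction script and maps the cursor to tile indices.
; SpawnGrid centers a snapped grid, stores tiles by index and pushes each to a child BP_GridVisuals actor.
; Optional sphere traces snap tile height to the ground and let BP_GridModifier actors set tile type.
; Cursor lookup uses a trace with plane-intersection fallback; world-to-index conversion handles only square shapes.
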(event `self.ReceiveBeginPlay`)

(fn `AddGridTile`
  (params (Data :type "/Game/BP/Core/Gride/Utilities/S_TileData Structure"))
  (bind _data_index (break `/Game/BP/Core/Gride/Utilities/S_TileData` (`local.Data`)))
  (`BlueprintMapLibrary.Map_Add` (`self.GridTiles`) _data_index (`local.Data`))
  (`/Game/BP/Core/Gride/Actor/BP_GridVisuals.Update Tile Visual` (`self.GridVisuals`) (`local.Data`)))

(fn `Calculate Center And Bottom Leeft`
  (returns (Center :type "Vector Structure") (`Bottom left` :type "Vector Structure"))
  (locals (C :type "Vector Structure" :default (0.0 0.0 0.0)))
  (bind (_gridtilecount_x _gridtilecount_y) (break `IntPoint` (`self.GridTileCount`)))
  (set `local.C` (`/Game/BP/Core/Utilities/BFL_utilities.Snap Vector to Vector` (`self.GridCenterLocation`) (`self.GrideTileSize`)))
  (return (`local.C`) (- (`local.C`) (`KismetMathLibrary.Conv_Vector2DToVector` (* (/ (- (`self.GridTileCount`) (`KismetMathLibrary.MakeVector2D` (`KismetMathLibrary.SelectFloat` 0.0 1.0 (`/Game/BP/Core/Utilities/BFL_utilities.IsFloatEven` (`KismetMathLibrary.Conv_IntToDouble` _gridtilecount_x))) (`KismetMathLibrary.SelectFloat` 0.0 1.0 (`/Game/BP/Core/Utilities/BFL_utilities.IsFloatEven` (`KismetMathLibrary.Conv_IntToDouble` _gridtilecount_y))))) (2.0 2.0)) (`KismetMathLibrary.Conv_VectorToVector2D` (`self.GrideTileSize`)))))))

(fn `DestroyGrid`
  (`BlueprintMapLibrary.Map_Clear` (`self.GridTiles`))
  (`/Game/BP/Core/Gride/Actor/BP_GridVisuals.DestrouGridVisual` (`self.GridVisuals`)))

(fn `Get Cursor Location On Grid`
  (params (PlayerIndex :type Integer))
  (returns (Location :type "Vector Structure"))
  (bind _returnvalue (`GameplayStatics.GetPlayerController` PlayerIndex))
  (bind (_hitresult _returnvalue_2) (`PlayerController.GetHitResultUnderCursorByChannel` _returnvalue "TraceTypeQuery4" false))
  (bind (_worldlocation _worlddirection) (`PlayerController.DeprojectMousePositionToWorld` _returnvalue))
  (bind (_t _intersection _returnvalue_3) (`KismetMathLibrary.LinePlaneIntersection` _worldlocation (+ _worldlocation (* _worlddirection 9999999.0)) (`KismetMathLibrary.MakePlaneFromPointAndNormal` (`self.GridCenterLocation`) (0.0 0.0 1.0))))
  (if _returnvalue_2
    (return (`.Location` (`GameplayStatics.BreakHitResult` _hitresult)))
    (elif _returnvalue_3
      (return _intersection)
      (else
        (return (-999.0 -999.0 -999.0))))))

(fn `Get Tile Index Under Cursor`
  (params (PlayerIndex :type Integer))
  (returns (Index :type "IntPoint Structure"))
  (bind _location (`self.Get Cursor Location On Grid` PlayerIndex))
  (bind _index (`self.Get Tile Index World Location` _location))
  (return _index))

(fn `Get Tile Index World Location`
  (params (Location :type "Vector Structure"))
  (returns (Index :type "IntPoint Structure"))
  (locals (LocationOnGrid :type "Vector Structure") (SnapLocationOnGrid :type "Vector2D Structure"))
  (set `local.LocationOnGrid` (- Location (`self.GridBottonLeftCornerLocation`)))
  (switch `/Game/BP/Core/Gride/GrideShapes/E_GridShape` (`self.GridShape`)
    (:`NewEnumerator0`
      (return (make `IntPoint` -999 -999)))
    (:`NewEnumerator1`
      (set `local.SnapLocationOnGrid` (`KismetMathLibrary.Conv_VectorToVector2D` (`/Game/BP/Core/Utilities/BFL_utilities.Snap Vector to Vector` (`local.LocationOnGrid`) (`self.GrideTileSize`))))
      (return (`KismetMathLibrary.Conv_Vector2DToIntPoint` (/ (`local.SnapLocationOnGrid`) (`KismetMathLibrary.Conv_VectorToVector2D` (`self.GrideTileSize`))))))))

(fn `GetCurrentShapeData`
  (returns (ReturnValue :type "/Game/BP/Core/Gride/GrideShapes/S_GridShapeData Structure"))
  (return (`/Game/BP/Core/Gride/GrideShapes/BFL_GridShape.GetShapeData` (`self.GridShape`))))

(fn `SetGridOffsetFromGround`
  (params (GridOffese :type "Float (double-precision)"))
  (set `self.Grid OffesetFromGround` GridOffese)
  (`SceneComponent.K2_SetWorldLocation` (`self.InstancedStaticMesh`) (`KismetMathLibrary.MakeVector` 0.0 0.0 (`self.Grid OffesetFromGround`)) false false))

(fn `SpawnGrid`
  (params (CenterLocation :type "Vector Structure") (TileSize :type "Vector Structure") (TileCount :type "IntPoint Structure") (Shape :type "/Game/BP/Core/Gride/GrideShapes/E_GridShape Enum" :default "NewEnumerator0") (UseEnvironment :type Boolean))
  (locals (x :type Integer) (Y :type Integer) (TileTransform :type "Transform Structure" :default "0.000000,0.000000,0.000000|0.000000,0.000000,-0.000000|1.000000,1.000000,1.000000") (Index :type "IntPoint Structure"))
  (bind (_tiletransform_location _tiletransform_rotation _tiletransform_scale) (`KismetMathLibrary.BreakTransform` (`local.TileTransform`)))
  (bind (_gridtilecount_x _gridtilecount_y) (break `IntPoint` (`self.GridTileCount`)))
  (bind _gridtilecount_x_2 (break `IntPoint` (`self.GridTileCount`)))
  (set `self.GridCenterLocation` CenterLocation)
  (set `self.GrideTileSize` TileSize)
  (set `self.GridShape` Shape)
  (set `self.GridTileCount` TileCount)
  (`self.DestroyGrid`)
  ;[1 1 1] visuel de la grille
  (`/Game/BP/Core/Gride/Actor/BP_GridVisuals.InitializeGridVisual` (`self.GridVisuals`) self)
  (bind (_center _bottom_left) (`self.Calculate Center And Bottom Leeft`))
  (set `self.GridCenterLocation` _center)
  (set `self.GridBottonLeftCornerLocation` _bottom_left)
  (for _index (range _gridtilecount_x_2)
    (set `local.x` _index)
    (for _index_2 (range (+ (- _gridtilecount_y 0) 1))
      (set `local.Y` _index_2)
      (set `local.Index` (make `IntPoint` (`local.x`) (`local.Y`)))
      (set `local.TileTransform` (`KismetMathLibrary.MakeTransform` (+ (+ (`self.GridBottonLeftCornerLocation`) (* (`self.GrideTileSize`) (`KismetMathLibrary.MakeVector` (`KismetMathLibrary.Conv_IntToDouble` (`local.x`)) (`KismetMathLibrary.Conv_IntToDouble` (`local.Y`))))) (0.0 0.0 2.0)) (struct) (/ (`self.GrideTileSize`) (`.MeshSize_2_681A6D26452BCC0223D1D484F8894336` (break `/Game/BP/Core/Gride/GrideShapes/S_GridShapeData` (`self.GetCurrentShapeData`))))))
      (if (`local.UseEnvironment`)
        (bind (_tiletype _outlocation) (`self.Trace for Ground` _tiletransform_location))
        (`self.AddGridTile` (make `/Game/BP/Core/Gride/Utilities/S_TileData` (`local.Index`) _tiletype (`KismetMathLibrary.MakeTransform` _outlocation _tiletransform_rotation _tiletransform_scale)))
        (else
          (`self.AddGridTile` (make `/Game/BP/Core/Gride/Utilities/S_TileData` (`local.Index`) "NewEnumerator1" (`local.TileTransform`))))))))

(fn `Trace for Ground`
  (params (Location :type "Vector Structure"))
  (returns (TileType :type "/Game/BP/Core/Gride/Utilities/E_TileType Enum") (OutLocation :type "Vector Structure"))
  (locals (RetType :type "/Game/BP/Core/Gride/Utilities/E_TileType Enum" :default "NewEnumerator1") (RetZ :type "Float (double-precision)" :default 0.0) (NewLocalVar_0 :type "Vector Structure" :default (0.0 0.0 0.0)))
  (bind _gridetilesize_x (`KismetMathLibrary.BreakVector` (`self.GrideTileSize`)))
  (bind _location (`local.Location`))
  (bind (_location_x _location_y) (`KismetMathLibrary.BreakVector` (`local.Location`)))
  (bind (_gridetilesize_x_2 _gridetilesize_y _gridetilesize_z) (`KismetMathLibrary.BreakVector` (`self.GrideTileSize`)))
  (set `self.Radius` (/ _gridetilesize_x 3.0))
  (bind _outhits (`KismetSystemLibrary.SphereTraceMulti` (+ _location (0.0 0.0 1000.0)) (- _location (0.0 0.0 0.0)) (`self.Radius`) "TraceTypeQuery3"))
  (if (> (`KismetArrayLibrary.Array_Length` _outhits) 0)
    (set `local.RetType` "NewEnumerator1")
    (for _array_element _outhits
      (bind (_bblockinghit _binitialoverlap _time _distance _location_2 _impactpoint _normal _impactnormal _physmat _hitactor) (`GameplayStatics.BreakHitResult` _array_element))
      (bind _asbp_grid_modifier (cast `/Game/BP/Core/Gride/Actor/BP_GridModifier` _hitactor)
        (:`then`
          (set `local.RetType` (`/Game/BP/Core/Gride/Actor/BP_GridModifier.Type` _asbp_grid_modifier)))
        (:`CastFailed`
          (set `local.RetZ` (`KismetMathLibrary.GridSnap_Float` (- (.z _location_2) (`self.Radius`)) _gridetilesize_z)))))
    (return (`local.RetType`) (`KismetMathLibrary.MakeVector` _location_x _location_y (`local.RetZ`)))
    (else
      (return "NewEnumerator0" (`local.Location`)))))

(fn `UserConstructionScript`
  (set `self.GridVisuals` (cast `/Game/BP/Core/Gride/Actor/BP_GridVisuals` (`ChildActorComponent.ChildActor` (`self.ChildActor_GridVisuals`)) :!pure true))
  (`self.SpawnGrid` (`self.K2_GetActorLocation`) (`self.GrideTileSize`) (`self.GridTileCount`) (`self.GridShape`) true))