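; BP_GridVisuals is the actor that draws the walkable tiles of a grid as mesh instances.
; On initialization it sets up a child BP_GridMeshinst with the grid shape's flat mesh and border material using query-only collision, then moves to the origin raised by a ground offset.
; Tile updates remove the instance at that index and re-add it only if the tile type is walkable.
; Destroying the visual clears all instances, and tick is disabled.
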(event `self.ReceiveBeginPlay`
  (`self.SetActorTickEnabled` false))

(fn `DestrouGridVisual`
  (bind _gridmeshint (`self.GridMeshInt`))
  (`/Engine/EditorBlueprintResources/StandardMacros.IsValid` _gridmeshint
    (:`Is Valid`
      (`/Game/BP/Core/Gride/Utilities/BP_GridMeshinst.ClearInstances` _gridmeshint))))

(fn `InitializeGridVisual`
  (params (Grid :type "/Game/BP/Core/Gride/Actor/BP_Grid Object Reference"))
  (bind (_meshsize _mesh _meshmaterial _flatmesh _flatbordermaterial) (break `/Game/BP/Core/Gride/GrideShapes/S_GridShapeData` (`/Game/BP/Core/Gride/Actor/BP_Grid.GetCurrentShapeData` (`self.Grid`))))
  (set `self.Grid` Grid)
  (bind _asbp_grid_meshinst (cast `/Game/BP/Core/Gride/Utilities/BP_GridMeshinst` (`ChildActorComponent.ChildActor` (`self.ChildActor_GridMeshInt`))))
  (set `self.GridMeshInt` _asbp_grid_meshinst)
  (`/Game/BP/Core/Gride/Utilities/BP_GridMeshinst.InitializeGridMeshinst` :`self` (`self.GridMeshInt`) :`Mesh` _flatmesh :`Material` _flatbordermaterial :`Collision` "QueryOnly")
  (`self.K2_SetActorLocation` (0.0 0.0 0.0))
  (`self.SeOffsetFromGround` (`self.Offset`)))

(fn `SeOffsetFromGround`
  (params (Offset :type "Float (double-precision)"))
  (bind (_returnvalue_x _returnvalue_y) (`KismetMathLibrary.BreakVector` (`self.K2_GetActorLocation`)))
  (set `self.Offset` Offset)
  (`self.K2_SetActorLocation` (`KismetMathLibrary.MakeVector` _returnvalue_x _returnvalue_y (`self.Offset`))))

(fn `Update Tile Visual`
  (params (Data :type "/Game/BP/Core/Gride/Utilities/S_TileData Structure"))
  (bind (_data_index _data_type _data_transform) (break `/Game/BP/Core/Gride/Utilities/S_TileData` (`local.Data`)))
  (bind (_data_index_2 _data_type_2) (break `/Game/BP/Core/Gride/Utilities/S_TileData` (`local.Data`)))
  (`/Game/BP/Core/Gride/Utilities/BP_GridMeshinst.RemoveINstance` (`self.GridMeshInt`) _data_index_2)
  (if (`/Game/BP/Core/Gride/Utilities/BFL_tiledata.Is Tile Type Walkable` _data_type_2)
    (`/Game/BP/Core/Gride/Utilities/BP_GridMeshinst.AddInstance` (`self.GridMeshInt`) _data_transform _data_index)))

(fn `UserConstructionScript`)